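; NPC actor that starts a dialogue when the third-person character enters its Box trigger.
; The overlap stores the player, switches its input mapping, clears all widgets and opens W_Dialogue with this NPC, its name and a starting index of zero.
; DestroyingPNJ runs a timeline that lerps the NPC toward the player's location and rotation while shrinking it to zero scale, without actually destroying the actor.
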(event `DestroyingPNJ`
  (bind (_returnvalue_location _returnvalue_rotation) (`KismetMathLibrary.BreakTransform` (`self.GetTransform` (`self.Player`))))
  (bind (_direction _alpha) (`Timeline|Timeline`)
    (:`Update`
      (`self.K2_SetActorTransform` (`KismetMathLibrary.TLerp` (`self.GetTransform`) (`KismetMathLibrary.MakeTransform` _returnvalue_location _returnvalue_rotation (0.0 0.0 0.0)) _alpha)))))

(event `self.Box.OnComponentBeginOverlap`
  (params (OverlappedComponent :type "PrimitiveComponent Object Reference") (OtherActor :type "Actor Object Reference") (OtherComp :type "PrimitiveComponent Object Reference") (OtherBodyIndex :type Integer) (bFromSweep :type Boolean) (SweepResult :type "HitResult Structure (by ref)"))
  (bind _asbp_third_person_character (cast `/Game/Blueprints/Character/BP_ThirdPersonCharacter` OtherActor))
  (set `self.Player` _asbp_third_person_character)
  (`/Game/Blueprints/Character/BP_ThirdPersonCharacter.SwitchMappingSystem` _asbp_third_person_character)
  (`WidgetLayoutLibrary.RemoveAllWidgets`)
  (bind _returnvalue (`|CreateWidget` "/Game/Blueprints/Widget/W_Dialogue.W_Dialogue_C" (`GameplayStatics.GetPlayerController` 0)))
  (set `/Game/Blueprints/Widget/W_Dialogue.PNJ` self _returnvalue)
  (set `/Game/Blueprints/Widget/W_Dialogue.ActualIndex` 0 _returnvalue)
  (`UserWidget.AddToViewport` _returnvalue 0)
  (set `EditableTextBox.Text` (`self.Name`) (`/Game/Blueprints/Widget/W_Dialogue.Text_Name` _returnvalue)))

(fn `UserConstructionScript`)