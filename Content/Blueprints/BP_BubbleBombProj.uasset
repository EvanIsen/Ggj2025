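; Bubble bomb projectile that sticks when it hits a cobweb or bubble puddle.
; The Bubble component's hit event class-checks the hit actor against BP_Cobweb and BP_BubblePuddle, ignoring other hits.
; On a match it zeroes physics velocity, widens the bubble on Y and Z, makes it block Pawns, and sets IsSticked.
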(event `self.Bubble.OnComponentHit`
  (params (HitComponent :type "PrimitiveComponent Object Reference") (OtherActor :type "Actor Object Reference") (OtherComp :type "PrimitiveComponent Object Reference") (NormalImpulse :type "Vector Structure") (Hit :type "HitResult Structure (by ref)"))
  (bind _bubble (`self.Bubble`))
  (bind _returnvalue (`GameplayStatics.GetObjectClass` (`.HitActor` (`GameplayStatics.BreakHitResult` Hit))))
  (if (`KismetMathLibrary.ClassIsChildOf` _returnvalue "/Game/Blueprints/BP_Cobweb.BP_Cobweb_C")
    (`PrimitiveComponent.SetPhysicsLinearVelocity` _bubble (0.0 0.0 0.0) false "None" :!label _label)
    (`SceneComponent.SetRelativeScale3D` _bubble (1.0 1.2 1.2))
    (`PrimitiveComponent.SetCollisionResponseToChannel` (`self.Bubble`) "ECC_Pawn" "ECR_Block")
    (set `self.isSticked` true)
    (elif (`KismetMathLibrary.ClassIsChildOf` _returnvalue "/Game/Blueprints/BP_BubblePuddle.BP_BubblePuddle_C")
      (goto _label))))

(fn `UserConstructionScript`)